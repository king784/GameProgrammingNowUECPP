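; Arena boundary Blueprint that pushes a player character when it overlaps one of four edge actors.
; Each edge's overlap event stores that edge's forward vector as StunDirection, then calls a shared check that casts to MyPlayerCharacter.
; A timeline restarts and each update applies that vector, scaled by its MoveValue track, as an unswept offset in the player's local space.
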(event `OverlapPlayerCheck`
  (params (OtherActor :type "Actor Object Reference"))
  (bind _asmy_player_character (cast `MyPlayerCharacter` OtherActor))
  (bind (_direction _movevalue) (`Timeline|MovePlayerTimeline` :!via `PlayFromStart`)
    (:`Update`
      (`self.K2_AddActorLocalOffset` _asmy_player_character (* (`self.StunDirection`) _movevalue) false false))))

(event `self.EdgeLeft.OnActorBeginOverlap`
  (params (OverlappedActor :type "Actor Object Reference") (OtherActor :type "Actor Object Reference"))
  (set `self.StunDirection` (`self.GetActorForwardVector` (`self.EdgeLeft`)))
  (`self.OverlapPlayerCheck` OtherActor))

(event `self.EdgeTop.OnActorBeginOverlap`
  (params (OverlappedActor :type "Actor Object Reference") (OtherActor :type "Actor Object Reference"))
  (set `self.StunDirection` (`self.GetActorForwardVector` (`self.EdgeTop`)))
  (`self.OverlapPlayerCheck` OtherActor))

(event `self.EdgeRight.OnActorBeginOverlap`
  (params (OverlappedActor :type "Actor Object Reference") (OtherActor :type "Actor Object Reference"))
  (set `self.StunDirection` (`self.GetActorForwardVector` (`self.EdgeRight`)))
  (`self.OverlapPlayerCheck` OtherActor))

(event `self.EdgeBottom.OnActorBeginOverlap`
  (params (OverlappedActor :type "Actor Object Reference") (OtherActor :type "Actor Object Reference"))
  (set `self.StunDirection` (`self.GetActorForwardVector` (`self.EdgeBottom`)))
  (`self.OverlapPlayerCheck` OtherActor))

(fn `UserConstructionScript`)