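; Enemy Blueprint that repeatedly fades its static mesh's material in and out; no other gameplay logic is implemented.
; BeginPlay applies a dynamic material instance to the mesh, then calls DoFade after a short delay.
; DoFade uses a FlipFlop to alternate the Fade timeline between forward and reverse playback.
; The timeline drives the material's Fade scalar parameter and calls DoFade on finishing, creating an endless ping-pong loop.
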(event `self.ReceiveBeginPlay`
  (bind _staticmeshcomponent (`self.StaticMeshComponent`))
  (bind _returnvalue (`KismetMaterialLibrary.CreateDynamicMaterialInstance` (`PrimitiveComponent.GetMaterial` _staticmeshcomponent 0)))
  (bind _output_get (set `self.Material` _returnvalue))
  (`PrimitiveComponent.SetMaterial` _staticmeshcomponent 0 _output_get)
  (`KismetSystemLibrary.Delay` 1.0)
  (`self.DoFade`))

(event `DoFade`
  (`/Engine/EditorBlueprintResources/StandardMacros.FlipFlop`
    (:`A`
      (bind (_direction _fade) (`Timeline|Fade` :!via `PlayFromStart` :!label _label)
        (:`Update`
          (`MaterialInstanceDynamic.SetScalarParameterValue` (`self.Material`) "Fade" _fade))
        (:`Finished`
          (`self.DoFade`))))
    (:`B`
      (goto _label :!via `ReverseFromEnd`))))

(fn `UserConstructionScript`)