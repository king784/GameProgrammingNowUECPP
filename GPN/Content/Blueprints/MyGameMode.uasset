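; Game mode that switches between main menu, playing and game over states, loading the matching level for the first two.
; On BeginPlay in TestLevel it caches the first level sequence actor and cine camera found.
; NotifyDead triggers a one-time game over, which moves the camera relative to the player, rotates and offsets the character, then plays the sequence.
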(event `NotifyInterface.NotifyDead`
  (params (Context :type "MyPlayerCharacter Object Reference"))
  (`self.ChangeState` "NewEnumerator2"))

(event `self.ReceiveBeginPlay`
  (bind _returnvalue (`GameplayStatics.GetCurrentLevelName` true))
  (if (`KismetStringLibrary.EqualEqual_StrStr` _returnvalue "TestLevel")
    (`/Engine/EditorBlueprintResources/StandardMacros.IsValid` (`self.GameOverSequence`)
      (:`Is Not Valid`
        (bind _outactors (`GameplayStatics.GetAllActorsOfClass` "/Script/LevelSequence.LevelSequenceActor"))
        (set `self.GameOverSequence` (`|GetArrayItem` _outactors))
        (bind _outactors_2 (`GameplayStatics.GetAllActorsOfClass` "/Script/CinematicCamera.CineCameraActor"))
        (set `self.CineCamActor` (`|GetArrayItem` _outactors_2))))))

(event `ChangeState`
  (params (GameEnum :type "/Game/Blueprints/GameState Enum" :default "NewEnumerator0"))
  (bind _cinecamactor (`self.CineCamActor`))
  (bind (_returnvalue_x _returnvalue_y _returnvalue_z) (`KismetMathLibrary.BreakVector` (`self.K2_GetActorLocation` _cinecamactor)))
  (`/Engine/EditorBlueprintResources/StandardMacros.IsValid` (`GameplayStatics.GetPlayerCharacter` 0)
    (:`Is Valid`
      _)
    (:`Is Not Valid`
      _))
  (switch `/Game/Blueprints/GameState` GameEnum
    (:`NewEnumerator0`
      (`GameplayStatics.OpenLevel` "Minimal_Default2"))
    (:`NewEnumerator1`
      (`GameplayStatics.OpenLevel` "TestLevel"))
    (:`NewEnumerator2`
      (if (not (`self.GameOverDone`))
        (set `self.GameOverDone` true)
        (bind _asmy_player_character (cast `MyPlayerCharacter` (`GameplayStatics.GetPlayerCharacter` 0)))
        (bind (_returnvalue_x_2 _returnvalue_y_2) (`KismetMathLibrary.BreakVector` (`self.K2_GetActorLocation` _asmy_player_character)))
        (`self.K2_SetActorLocation` _cinecamactor (`KismetMathLibrary.MakeVector` (+ _returnvalue_x_2 1020.0) (+ _returnvalue_y_2 500.0) _returnvalue_z) false false)
        (`self.K2_AddActorWorldRotation` _asmy_player_character (struct :`Pitch` 90.0) false false)
        (`self.K2_AddActorLocalOffset` _asmy_player_character (0.0 0.0 400.0) false false)
        (`MovieSceneSequencePlayer.Play` (`LevelSequenceActor.SequencePlayer` (`self.GameOverSequence`)))))))

(fn `UserConstructionScript`)