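; Portal actor with an eye that aims at the player, fires a LaserBall, then shrinks away and destroys itself.
; A chain of timelines and delays from BeginPlay scales the portal, moves and rotates the eye, plays the EyeLaser charge emitter, then spawns the projectile along the eye's forward vector.
; Tick smoothly turns the eye toward player 0 while Mode is 1, stopping once the shot spawns.
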(event `self.ReceiveBeginPlay`
  (`self.ScalePortal` true))

(event `ScalePortal`
  (params (Bigger :type Boolean))
  (bind _eye (`self.Eye`))
  (bind _returnvalue_location (`KismetMathLibrary.BreakTransform` (`SceneComponent.K2_GetComponentToWorld` _eye)))
  (if Bigger
    (bind (_direction _newtrack_0) (`Timeline|Timeline_0` :!via `ReverseFromEnd`)
      (:`Update`
        (`self.SetActorScale3D` _newtrack_0))
      (:`Finished`
        (`KismetSystemLibrary.Delay` 0.2)
        (bind (_direction_2 _moveeye) (`Timeline|MoveEye` :!via `PlayFromStart`)
          (:`Update`
            (`SceneComponent.K2_AddLocalOffset` (`self.Eye`) (`KismetMathLibrary.MakeVector` _moveeye) false false))
          (:`Finished`
            (`KismetSystemLibrary.Delay` 0.15)
            (bind (_direction_3 _rotation) (`Timeline|RotateEye` :!via `PlayFromStart`)
              (:`Update`
                (`SceneComponent.K2_AddLocalRotation` (`self.Eye`) (`KismetMathLibrary.MakeRotator` (.x _rotation) (.y _rotation) (.z _rotation)) false false))
              (:`Finished`
                (set `self.Mode` 1)
                (`KismetSystemLibrary.Delay` 2.0)
                (bind _returnvalue (`GameplayStatics.SpawnEmitterAtLocation` "/Game/particles/EyeLaser.EyeLaser" (`SceneComponent.K2_GetComponentLocation` (`self.ParticleSpawnPoint`)) (struct) (1.0 1.0 1.0) false))
                (`KismetSystemLibrary.Delay` 1.8)
                (`ActorComponent.Deactivate` _returnvalue)
                (`KismetSystemLibrary.Delay` 0.2)
                (`|SpawnActorFromClass` "/Game/Blueprints/LaserBall.LaserBall_C" (`KismetMathLibrary.MakeTransform` (+ _returnvalue_location (* (`SceneComponent.GetForwardVector` _eye) 200.0)) (`SceneComponent.K2_GetComponentRotation` (`self.Eye`))) "AdjustIfPossibleButAlwaysSpawn" "OverrideRootScale" null null)
                (set `self.Mode` 0)
                (bind (_direction_4 _pitchval) (`Timeline|EyeRotEnd` :!via `PlayFromStart`)
                  (:`Update`
                    (`SceneComponent.K2_AddLocalRotation` (`self.Eye`) (`KismetMathLibrary.MakeRotator` 0.0 _pitchval) false false))
                  (:`Finished`
                    (`self.ScalePortal` false)))))))))
    (else
      (bind (_direction_5 _newtrack_0_2) (`Timeline|ScaleTimeline` :!via `PlayFromStart`)
        (:`Update`
          (`self.SetActorScale3D` _newtrack_0_2))
        (:`Finished`
          (`self.K2_DestroyActor`))))))

(event `self.ReceiveTick`
  (params (DeltaSeconds :type "Float (single-precision)"))
  (bind _eye (`self.Eye`))
  (switch `int` (`self.Mode`)
    (:`1`
      (bind _asmy_player_character (cast `MyPlayerCharacter` (`GameplayStatics.GetPlayerCharacter` 0)))
      (`SceneComponent.K2_SetWorldRotation` _eye (`KismetMathLibrary.RInterpTo` (`SceneComponent.K2_GetComponentRotation` _eye) (`KismetMathLibrary.FindLookAtRotation` (`SceneComponent.K2_GetComponentLocation` _eye) (`self.K2_GetActorLocation` _asmy_player_character)) DeltaSeconds 3.0) false false))))

(fn `UserConstructionScript`)