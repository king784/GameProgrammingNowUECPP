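; Robot is a temporary pursuer actor that follows the player and drains battery charge on capsule overlap.
; Each tick it eases toward a point just ahead of the player with VInterpTo, clamps its height above a minimum and faces the player.
; A timeline drives its scale on spawn, then after a delay Deactivate plays a second scale timeline in reverse and destroys the actor.
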(event `self.ReceiveBeginPlay`
  (bind (_direction _scale) (`Timeline|Timeline_0` :!via `PlayFromStart`)
    (:`Update`
      (`self.SetActorScale3D` (`KismetMathLibrary.MakeVector` _scale _scale _scale)))
    (:`Finished`
      (`KismetSystemLibrary.Delay` 6.0)
      (`self.Deactivate`))))

(event `self.ReceiveTick`
  (params (DeltaSeconds :type "Float (single-precision)"))
  (bind _returnvalue (`self.K2_GetActorLocation`))
  (bind _asmy_player_character (cast `MyPlayerCharacter` (`GameplayStatics.GetPlayerCharacter` 0)))
  (bind _returnvalue_2 (`self.K2_GetActorLocation` _asmy_player_character))
  (bind (_returnvalue_x _returnvalue_y _returnvalue_z) (`KismetMathLibrary.BreakVector` (`KismetMathLibrary.VInterpTo` _returnvalue (+ _returnvalue_2 (* (`self.GetActorForwardVector` _asmy_player_character) 1.0)) DeltaSeconds 1.0)))
  (`self.K2_SetActorLocationAndRotation` (`KismetMathLibrary.MakeVector` _returnvalue_x _returnvalue_y (`KismetMathLibrary.FClamp` _returnvalue_z 200.0 100000.0)) (`KismetMathLibrary.FindLookAtRotation` _returnvalue _returnvalue_2)))

(event `self.CapsuleComponent.OnComponentBeginOverlap`
  (params (OverlappedComponent :type "PrimitiveComponent Object Reference") (OtherActor :type "Actor Object Reference") (OtherComp :type "PrimitiveComponent Object Reference") (OtherBodyIndex :type Integer) (bFromSweep :type Boolean) (SweepResult :type "HitResult Structure (by ref)"))
  (bind _asmy_player_character (cast `MyPlayerCharacter` OtherActor))
  (`MyPlayerCharacter.UpdateBatteryCharge` _asmy_player_character -1.1))

(event `Deactivate`
  (bind (_direction _scale) (`Timeline|Timeline_1` :!via `ReverseFromEnd`)
    (:`Update`
      (`self.SetActorScale3D` (`KismetMathLibrary.MakeVector` _scale _scale _scale)))
    (:`Finished`
      (`self.K2_DestroyActor`))))

(fn `UserConstructionScript`)