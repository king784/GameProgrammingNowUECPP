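; BadPickup is a temporary harmful pickup that drains the player's battery charge.
; On BeginPlay, a reversed timeline animates actor scale, then after a delay a second scale timeline plays and destroys the actor on finish.
; Box overlap with MyPlayerCharacter applies a negative battery update without destroying the pickup, so re-entering can drain charge again.
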(event `self.ReceiveBeginPlay`
  (bind (_direction _scale) (`Timeline|Timeline_1` :!via `ReverseFromEnd`)
    (:`Update`
      (`self.SetActorScale3D` _scale))
    (:`Finished`
      (`KismetSystemLibrary.Delay` 8.0)
      (bind (_direction_2 _scale_2) (`Timeline|ScaleTimeline_0` :!via `PlayFromStart`)
        (:`Update`
          (`self.SetActorScale3D` _scale_2))
        (:`Finished`
          (`self.K2_DestroyActor`))))))

(event `self.BoxCollision.OnComponentBeginOverlap`
  (params (OverlappedComponent :type "PrimitiveComponent Object Reference") (OtherActor :type "Actor Object Reference") (OtherComp :type "PrimitiveComponent Object Reference") (OtherBodyIndex :type Integer) (bFromSweep :type Boolean) (SweepResult :type "HitResult Structure (by ref)"))
  (bind _asmy_player_character (cast `MyPlayerCharacter` OtherActor))
  (`MyPlayerCharacter.UpdateBatteryCharge` _asmy_player_character -0.25))

(fn `UserConstructionScript`
  (`parent.UserConstructionScript`))