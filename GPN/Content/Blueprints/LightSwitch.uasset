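; LightSwitch is an interactable switch that turns a set of lights on and off.
; Its Interact event loops over the Lights array, casts each element to Light and toggles that light component's visibility.
; A Box overlap shows a TextRender when MyPlayerCharacter enters and hides it when the player leaves.
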(event `/Game/Blueprints/InteractI.Interact`
  (for _array_element (`self.Lights`)
    (bind _aslight (cast `Light` _array_element))
    (`SceneComponent.ToggleVisibility` (`Light.LightComponent` _aslight) false)))

(event `self.Box.OnComponentBeginOverlap`
  (params (OverlappedComponent :type "PrimitiveComponent Object Reference") (OtherActor :type "Actor Object Reference") (OtherComp :type "PrimitiveComponent Object Reference") (OtherBodyIndex :type Integer) (bFromSweep :type Boolean) (SweepResult :type "HitResult Structure (by ref)"))
  (cast `MyPlayerCharacter` OtherActor)
  (`SceneComponent.SetVisibility` (`self.TextRender`) true false))

(event `self.Box.OnComponentEndOverlap`
  (params (OverlappedComponent :type "PrimitiveComponent Object Reference") (OtherActor :type "Actor Object Reference") (OtherComp :type "PrimitiveComponent Object Reference") (OtherBodyIndex :type Integer))
  (cast `MyPlayerCharacter` OtherActor)
  (`SceneComponent.SetVisibility` (`self.TextRender`) false false))

(fn `UserConstructionScript`)