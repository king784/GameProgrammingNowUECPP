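; Player character Blueprint that lets the player interact with nearby actors implementing the InteractI interface.
; Capsule overlap events store the most recently entered interactable in InteractObj and clear it when any interactable leaves the capsule.
; Pressing the Interact input sends InteractMessage to the stored actor if it is valid, leaving the response to that actor.
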(event `InputAction|Interact`
  (params (Key :type "Key Structure"))
  (bind _interactobj (`self.InteractObj`))
  (:`Pressed`
    (`/Engine/EditorBlueprintResources/StandardMacros.IsValid` _interactobj
      (:`Is Valid`
        (message `/Game/Blueprints/InteractI.Interact` _interactobj)))))

(event `self.CapsuleComponent.OnComponentBeginOverlap`
  (params (OverlappedComponent :type "PrimitiveComponent Object Reference") (OtherActor :type "Actor Object Reference") (OtherComp :type "PrimitiveComponent Object Reference") (OtherBodyIndex :type Integer) (bFromSweep :type Boolean) (SweepResult :type "HitResult Structure (by ref)"))
  (if (`KismetSystemLibrary.DoesImplementInterface` OtherActor "/Game/Blueprints/InteractI.InteractI_C")
    (set `self.InteractObj` OtherActor)))

(event `self.CapsuleComponent.OnComponentEndOverlap`
  (params (OverlappedComponent :type "PrimitiveComponent Object Reference") (OtherActor :type "Actor Object Reference") (OtherComp :type "PrimitiveComponent Object Reference") (OtherBodyIndex :type Integer))
  (if (`KismetSystemLibrary.DoesImplementInterface` OtherActor "/Game/Blueprints/InteractI.InteractI_C")
    (set `self.InteractObj` null)))

(fn `UserConstructionScript`)