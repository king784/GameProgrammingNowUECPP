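; Laser spawner that periodically spawns a Laser actor on a random edge of a rectangular area marked by the TopLeft and BottomRight actors.
; BeginPlay starts a looping timer whose random interval is rolled only once, so the cadence stays constant afterwards.
; Each tick of the timer picks one of four sides, randomizes position along that padded edge at a fixed height, and sets a per-side yaw.
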(event `self.ReceiveBeginPlay`
  (`KismetSystemLibrary.K2_SetTimerDelegate` (delegate `SpawnLaser`) (`KismetMathLibrary.RandomFloatInRange` 6.0 10.0) true))

(event `SpawnLaser`
  (bind _returnvalue_x (`KismetMathLibrary.BreakVector` (`self.K2_GetActorLocation` (`self.TopLeft`))))
  (bind (_returnvalue_x_2 _returnvalue_y) (`KismetMathLibrary.BreakVector` (`self.K2_GetActorLocation` (`self.BottomRight`))))
  (bind (_returnvalue_x_3 _returnvalue_y_2) (`KismetMathLibrary.BreakVector` (`self.K2_GetActorLocation` (`self.TopLeft`))))
  (bind (_returnvalue_x_4 _returnvalue_y_3) (`KismetMathLibrary.BreakVector` (`self.K2_GetActorLocation` (`self.TopLeft`))))
  (bind _returnvalue_x_5 (`KismetMathLibrary.BreakVector` (`self.K2_GetActorLocation` (`self.BottomRight`))))
  (bind (_returnvalue_x_6 _returnvalue_y_4) (`KismetMathLibrary.BreakVector` (`self.K2_GetActorLocation` (`self.BottomRight`))))
  (bind (_returnvalue_x_7 _returnvalue_y_5) (`KismetMathLibrary.BreakVector` (`self.K2_GetActorLocation` (`self.TopLeft`))))
  (bind (_returnvalue_x_8 _returnvalue_y_6) (`KismetMathLibrary.BreakVector` (`self.K2_GetActorLocation` (`self.BottomRight`))))
  (switch `int` (`KismetMathLibrary.RandomIntegerInRange` 0 3)
    (:`0`
      ;[1 1 1] Spawn On Left Side
      (`|SpawnActorFromClass` "/Game/Blueprints/Laser.Laser_C" (`KismetMathLibrary.MakeTransform` (`KismetMathLibrary.MakeVector` (`KismetMathLibrary.RandomFloatInRange` (- _returnvalue_x_5 1000.0) (+ _returnvalue_x_4 1000.0)) _returnvalue_y_3 546.0) (struct :`Yaw` -180.0)) "Undefined" "OverrideRootScale" null null))
    (:`1`
      ;[1 1 1] Spawn On Top Side
      (`|SpawnActorFromClass` "/Game/Blueprints/Laser.Laser_C" (`KismetMathLibrary.MakeTransform` (`KismetMathLibrary.MakeVector` _returnvalue_x_7 (`KismetMathLibrary.RandomFloatInRange` (- _returnvalue_y_5 1000.0) (+ _returnvalue_y_6 1000.0)) 546.0) (struct :`Yaw` -90.0)) "Undefined" "OverrideRootScale" null null))
    (:`2`
      ;[1 1 1] Spawn On Right Side
      (`|SpawnActorFromClass` "/Game/Blueprints/Laser.Laser_C" (`KismetMathLibrary.MakeTransform` (`KismetMathLibrary.MakeVector` (`KismetMathLibrary.RandomFloatInRange` (- _returnvalue_x_2 1000.0) (+ _returnvalue_x 1000.0)) _returnvalue_y 546.0)) "Undefined" "OverrideRootScale" null null))
    (:`3`
      ;[1 1 1] Spawn On Bottom Side
      (`|SpawnActorFromClass` "/Game/Blueprints/Laser.Laser_C" (`KismetMathLibrary.MakeTransform` (`KismetMathLibrary.MakeVector` _returnvalue_x_6 (`KismetMathLibrary.RandomFloatInRange` (- _returnvalue_y_2 1000.0) (+ _returnvalue_y_4 1000.0)) 546.0) (struct :`Yaw` 90.0)) "Undefined" "OverrideRootScale" null null))))

(fn `UserConstructionScript`)